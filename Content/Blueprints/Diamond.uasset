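; Diamond is a collectible falling under a parent class's logic, reused by resetting its position, scale and value after any overlap.
; On overlap it checks the other actor's object name for a Peikko hit, then broadcasts DiamondCollectedED with its Value and plays a sound.
; Otherwise it runs the respawn-trigger check.
; Tick only calls the parent, and ApllyEffect is empty.
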(event EventBeginPlay)

(event Collision|EventActorBeginOverlap
  (params (OtherActor :type Actor%20Object%20Reference))
  (bind _returnvalue (Utilities|GetObjectName OtherActor))
  ;[1 1 1] Check if diamond hit peikko and play sound
  (bind _hitresult (CallFunction|CheckPeikkoHit _returnvalue))
  (if _hitresult
    ;[1 1 1] Broeadcast message that money was collected by peikko
    (Default|CallDiamondCollectedED (Variables|Default|GetValue))
    (Audio|PlaySound2D "/Game/Sounds/Collect_good_sound.Collect_good_sound" 1.0 1.0 0.0 0 0)
    (else
      ;[1 1 1] if not peikko, check if we hit respawn trigger
      (CallFunction|CheckRespawnHit _returnvalue)))
  ;[1 1 1] reset diamond values
  (CallFunction|ResetPosition)
  (CallFunction|ResetScaleandValue))

(event EventTick
  (params (DeltaSeconds :type Float%20%28single-precision%29))
  (|CallParentFunction 0.0))

(fn ConstructionScript)

(fn ApllyEffect)