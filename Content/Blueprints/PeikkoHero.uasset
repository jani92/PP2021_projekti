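; PeikkoHero is the player character Blueprint, handling movement, jumping and pausing.
; The Move_right axis drives movement along world X, and W starts and stops a jump.
; P creates the PauseMenu widget once and reuses it, then shows the cursor, switches to UI-only input and pauses the game.
; BeginPlay restores game-only input.
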(event EventBeginPlay
  (Input|SetInputModeGameOnly (Game|GetPlayerController 0)))

(event Collision|EventActorBeginOverlap
  (params (OtherActor :type Actor%20Object%20Reference)))

(event EventTick
  (params (DeltaSeconds :type Float%20%28single-precision%29)))

(event Input|AxisEvents|InputAxisMove_right
  (params (AxisValue :type Float%20%28single-precision%29))
  (Pawn|Input|AddMovementInput "1.000000, 0, 0" AxisValue false))

(event Input|KeyboardEvents|W
  (params (Key :type Key%20Structure :default "None"))
  (:Pressed
    (Character|Jump))
  (:Released
    (Character|StopJumping)))

(event Input|KeyboardEvents|P
  (params (Key :type Key%20Structure :default "None"))
  (bind _returnvalue (Game|GetPlayerController 0))
  (:Pressed
    (Utilities|IsValid (Variables|Default|GetPause%20Menu%20Reference)
      (:Is%20Valid
        _)
      (:Is%20Not%20Valid
        (bind _returnvalue_2 (UserInterface|CreateWidget "/Game/Blueprints/PauseMenu.PauseMenu_C"))
        (Variables|Default|SetPause%20Menu%20Reference _returnvalue_2)))
    (Variables|/Script/Engine.PlayerController|SetbShowMouseCursor _returnvalue true)
    (Input|SetInputModeUIOnly _returnvalue (Variables|Default|GetPause%20Menu%20Reference) "DoNotLock")
    (UserInterface|Viewport|AddtoViewport (Variables|Default|GetPause%20Menu%20Reference) 0)
    (Game|SetGamePaused true)))

(fn ConstructionScript)