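; Collectible actor that moves every tick by a Speed offset multiplied by global time dilation, not delta time.
; Reset functions return it to a stored start point with random height or to a fixed location, and set value from scale, whose random range is currently fixed.
; Name-comparison helpers identify hits on the player character ("Peikko") or respawn trigger.
; ApplyEffect, DelayAndPosition and ResetPositionPommi are empty stubs, and nothing here calls the helpers.
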(event EventBeginPlay)

(event Collision|EventActorBeginOverlap
  (params (OtherActor :type Actor%20Object%20Reference)))

(event EventTick
  (params (DeltaSeconds :type Float%20%28single-precision%29))
  ;[1 1 1] Move the collectible
  (Transformation|AddActorWorldOffset (* (Variables|Default|Getspeed) (Class|GameplayStatics|GetGlobalTimeDilation))))

(fn ConstructionScript)

(fn ResetPosition
  (bind _initialposition (Variables|Default|GetInitialPosition))
  (bind (_x _y) (Math|Vector|BreakVector _initialposition))
  (Transformation|SetActorLocation (Math|Vector|MakeVector _x _y (Math|Random|RandomFloatinRange 1e+02 4e+02)) false false))

(fn ResetScaleandValue
  (bind _output_get (Variables|Default|SetScale (Math|Random|RandomFloatinRange 1.0 1.0)))
  (Transformation|SetActorScale3D (Math|Vector|MakeVector (/ _output_get 1.0) (/ _output_get 1.0) (/ _output_get 1.0)))
  (Variables|Default|SetValue (Math|Float|Round (Variables|Default|GetScale))))

(fn CheckPeikkoHit
  (params (OtherObjectName :type String))
  (return (Utilities|Enum|Equal(Enum) OtherObjectName (Utilities|GetObjectName (Game|GetPlayerCharacter 0)))))

(fn CheckRespawnHit
  (params (OtherObjectName :type String))
  (return (Utilities|Enum|Equal(Enum) OtherObjectName (Variables|Default|GetRespawnTriggerName))))

(fn ResetPosition2
  (Transformation|SetActorLocation "1300.000000, 0,80.000000" false false))

(fn ResetPosition3
  (bind _initialpositionpommi (Variables|Default|GetinitialPositionPommi))
  (bind (_x _y) (Math|Vector|BreakVector _initialpositionpommi))
  (Transformation|SetActorLocation (Math|Vector|MakeVector _x _y (Math|Random|RandomFloatinRange 2e+02 3.5e+02)) false false))

(fn ResetPositionPommi)

(fn DelayandPosition)

(fn ApplyEffect)