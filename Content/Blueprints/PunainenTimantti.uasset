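; PunainenTimantti is a red diamond pickup that shrinks the player character when collected.
; On overlap, a Peikko hit triggers the collected event dispatcher on Koira and scales the player down; other actors go through a respawn check.
; It then teleports itself away and, after a delay, calls ResetPosition and ResetScaleAndValue.
; Tick only forwards to the parent class.
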(event EventBeginPlay)

(event Collision|EventActorBeginOverlap
  (params (OtherActor :type Actor%20Object%20Reference))
  (bind _returnvalue (Utilities|GetObjectName OtherActor))
  (bind _hitresult (CallFunction|CheckPeikkoHit _returnvalue))
  (if _hitresult
    (Default|CallPunainenTimanttiCollectedED (Variables|Default|GetKoira))
    (Transformation|SetActorScale3D (Game|GetPlayerCharacter 0) "0.300000,0.300000,0.300000")
    (else
      (CallFunction|CheckRespawnHit _returnvalue)))
  (Transformation|SetActorLocation "-2000.000000, 0, 0" false false)
  (Utilities|FlowControl|Delay 5.0)
  (CallFunction|ResetPosition)
  (CallFunction|ResetScaleandValue))

(event EventTick
  (params (DeltaSeconds :type Float%20%28single-precision%29))
  (|CallParentFunction 0.0))

(fn ConstructionScript)