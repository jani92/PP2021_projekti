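; Pommi is a collectible actor, apparently a bomb, that reports to Koira when picked up and recycles itself.
; On overlap, a name-based Peikko check triggers the collected call, teleports it to a fixed X with random height, then resets scale and value.
; Other overlaps run the respawn check, then reset position regardless of its result.
; Tick defers to the parent; its own leftward movement node is disconnected.
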(event EventBeginPlay)

(event Collision|EventActorBeginOverlap
  (params (OtherActor :type Actor%20Object%20Reference))
  (bind _returnvalue (Utilities|GetObjectName OtherActor))
  (bind _hitresult (CallFunction|CheckPeikkoHit _returnvalue))
  (if _hitresult
    (Default|CallPommiCollected (Variables|Default|GetKoira))
    (Transformation|SetActorLocation (Math|Vector|MakeVector 3e+03 0.0 (Math|Random|RandomFloatinRange 2e+02 4e+02)) false false)
    (CallFunction|ResetScaleandValue)
    (else
      (CallFunction|CheckRespawnHit _returnvalue)
      (CallFunction|ResetPosition3))))

(event EventTick
  (params (DeltaSeconds :type Float%20%28single-precision%29))
  (|CallParentFunction 0.0))

(fn ConstructionScript)