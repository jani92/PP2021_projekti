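; Kivii is a moving obstacle actor (kivi is Finnish for rock) that hits the player character and recycles to a start point.
; Tick offsets it by Speed2 scaled by global time dilation, without delta time.
; A player overlap, matched by object name, calls the HitByKiviEDD dispatcher with Value, resets position and sets Value to -1.
; Any other overlap also resets it, as the respawn trigger check's result goes unused.
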(event OnComponentBeginOverlap(Box)
  (params (OverlappedComponent :type Primitive%20Component%20Object%20Reference) (OtherActor :type Actor%20Object%20Reference) (OtherComp :type Primitive%20Component%20Object%20Reference) (OtherBodyIndex :type Integer) (bFromSweep :type Boolean) (SweepResult :type Hit%20Result%20Structure%20%28by%20ref%29)))

(event EventBeginPlay
  (|CallParentFunction) ; This node is disabled and will not be called.\nDrag off pins to build functionality.
)

(event EventTick
  (params (DeltaSeconds :type Float%20%28single-precision%29))
  (Transformation|AddActorWorldOffset (* (Variables|Default|GetSpeed2) (Class|GameplayStatics|GetGlobalTimeDilation))))

(event Collision|EventActorBeginOverlap
  (params (OtherActor :type Actor%20Object%20Reference))
  (bind _returnvalue (Utilities|GetObjectName OtherActor))
  (bind _hitresult (CallFunction|PeikkoHit _returnvalue))
  (if _hitresult
    (Default|CallHitbyKiviEDD (Variables|Default|Getvalue))
    (CallFunction|ResetPosition2)
    (CallFunction|SetValue)
    (else
      (CallFunction|RespawnHit _returnvalue)
      (Development|PrintString "huhu")
      (CallFunction|ResetPosition2))))

(fn ConstructionScript
  (|CallParentFunction))

(fn RespawnHit
  (params (OtherObjectName2 :type String))
  (return (Utilities|Enum|Equal(Enum) OtherObjectName2 (Variables|Default|GetRespawnTriggerName2))))

(fn PeikkoHit
  (params (OtherObjectName2 :type String))
  (return (Utilities|Enum|Equal(Enum) OtherObjectName2 (Utilities|GetObjectName (Game|GetPlayerCharacter 0)))))

(fn ResetPosition2
  (Transformation|SetActorLocation "1300.000000, 0,80.000000" false false))

(fn SetValue
  (Variables|Default|Setvalue -1))

(fn ApplyEffect
  (Development|PrintString "asdasdadasdas"))