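; Dead tree ("kuollutpuu") 2D obstacle that reacts when the player character ("peikko") overlaps it.
; A player hit, matched by object name, calls the HitByPuu dispatcher with Value, plays a slap sound and briefly swaps flipbooks.
; Any other overlap teleports the tree to a hard-coded position, as the RespawnHit name check's result is unused.
; SetValue and the debug-print ApplyEffect are not called here.
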(event EventBeginPlay
  (|CallParentFunction) ; This node is disabled and will not be called.\nDrag off pins to build functionality.
)

(event EventTick
  (params (DeltaSeconds :type Float%20%28single-precision%29))
  (|CallParentFunction DeltaSeconds))

(event Collision|EventActorBeginOverlap
  (params (OtherActor :type Actor%20Object%20Reference))
  (bind _returnvalue (Utilities|GetObjectName OtherActor))
  ;[1 1 1] Handle peikko hit event
  (bind _hitresult (CallFunction|PeikkoHit _returnvalue))
  (if _hitresult
    ;[1 1 1] If hit by puu make animation and handle event
    (Default|CallHitbyPuuED (Variables|Default|Getvalue))
    (Audio|PlaySound2D "/Game/Sounds/Slap_sound.Slap_sound" 1.0 1.0 0.0 0 0)
    (Sprite|SetFlipbook (Variables|Default|GetRenderComponent) "/Game/Flipbooks/kuollutpuu1.kuollutpuu1")
    (Utilities|FlowControl|Delay 0.7)
    (Sprite|SetFlipbook (Variables|Default|GetRenderComponent) "/Game/Flipbooks/kuollutpuu2.kuollutpuu2")
    (else
      ;[1 1 1] If respawn hit reset position
      (CallFunction|RespawnHit _returnvalue)
      (CallFunction|ResetPosition2))))

(fn ConstructionScript
  (|CallParentFunction))

(fn RespawnHit
  (params (OtherObjectName2 :type String))
  (return (Utilities|Enum|Equal(Enum) OtherObjectName2 (Variables|Default|GetRespawnTriggerName2))))

(fn PeikkoHit
  (params (OtherObjectName2 :type String))
  (return (Utilities|Enum|Equal(Enum) OtherObjectName2 (Utilities|GetObjectName (Game|GetPlayerCharacter 0)))))

(fn ResetPosition2
  (Transformation|SetActorLocation "1800.000000, 0,195.000000" false false))

(fn SetValue
  (Variables|Default|Setvalue -1))

(fn ApplyEffect
  (Development|PrintString "asdasdadasdas"))