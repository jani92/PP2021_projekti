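; CollectibleFlipBook is a collectible actor that moves through the world, with helpers for detecting hits and resetting its position.
; Tick offsets it by Speed times global time dilation, without delta seconds, so movement depends on frame rate.
; CheckPeikkoHit and CheckRespawnHit compare a supplied object name against the player character and the respawn trigger.
; ResetPosition returns it to InitialPosition; no graph here calls these helpers.
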(event EventBeginPlay)

(event Collision|EventActorBeginOverlap
  (params (OtherActor :type Actor%20Object%20Reference)))

(event EventTick
  (params (DeltaSeconds :type Float%20%28single-precision%29))
  ;[1 1 1] Move the collectible
  (Transformation|AddActorWorldOffset (* (Variables|Default|GetSpeed) (Class|GameplayStatics|GetGlobalTimeDilation))))

(fn ConstructionScript)

(fn ResetPosition
  (Transformation|SetActorLocation (Variables|Default|GetInitialPosition) false false))

(fn CheckPeikkoHit
  (params (OtherObjectName :type String))
  (return (Utilities|Enum|Equal(Enum) OtherObjectName (Utilities|GetObjectName (Game|GetPlayerCharacter 0)))))

(fn CheckRespawnHit
  (params (OtherObjectName :type String))
  (return (Utilities|Enum|Equal(Enum) OtherObjectName (Variables|Default|GetRespawnTriggerName))))